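; MovementTestBP is a controllable pawn for testing movement, with axis-driven walking and turning.
; Forward and sideways input move it relative to control yaw only, scaled by MoveSpeed, while Yaw input turns the controller by RotSpeed.
; The IsScared flag blocks all three inputs.
; SwitchedTo sets player 0's view target to CurrentCamera.
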(event `InputAxis|MoveForward`
  (params (AxisValue :type "Float (single-precision)"))
  ;[1 1 1] Character Controller
  ;;[1 1 1] Movement
  (if (not (`self.isScared`))
    (`self.AddMovementInput` (`KismetMathLibrary.GetForwardVector` (`KismetMathLibrary.MakeRotator` 0.0 0.0 (.yaw (`self.GetControlRotation`)))) (* AxisValue (`self.moveSpeed`)))))

(event `InputAxis|MoveSideways`
  (params (AxisValue :type "Float (single-precision)"))
  ;[1 1 1] Character Controller
  ;;[1 1 1] Movement
  (if (not (`self.isScared`))
    (`self.AddMovementInput` (`KismetMathLibrary.GetRightVector` (`KismetMathLibrary.MakeRotator` 0.0 0.0 (.yaw (`self.GetControlRotation`)))) (* (`self.moveSpeed`) AxisValue))))

(event `InputAxis|Yaw`
  (params (AxisValue :type "Float (single-precision)"))
  ;[1 1 1] Character Controller
  ;;[1 1 1] Rotation
  (if (not (`self.isScared`))
    (`self.AddControllerYawInput` (* AxisValue (`self.rotSpeed`)))))

(fn `SwitchedTo`
  (`PlayerController.SetViewTargetWithBlend` (`GameplayStatics.GetPlayerController` 0) (`self.currentCamera`) 0.0 "VTBlend_Linear" 0.0 false))

(fn `UserConstructionScript`)