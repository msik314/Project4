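; DarkKidBP is a kid actor that becomes scared when no MovementTestBP actor is close to it.
; Each Tick it sets IsScared, then scans all MovementTestBP actors and clears the flag at the first one within ScaredRadius.
; A math expression node does the distance test and ignores any actor at the same position, which would exclude itself.
; Nothing in this graph acts on the flag.
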(event EventBeginPlay
  (|CallParentFunction) ; This node is disabled and will not be called.\nDrag off pins to build functionality.
)

(event Collision|EventActorBeginOverlap
  (params (OtherActor :type Actor%20Object%20Reference))
  (|CallParentFunction OtherActor) ; This node is disabled and will not be called.\nDrag off pins to build functionality.
)

(event EventTick
  (params (DeltaSeconds :type Float%20%28single-precision%29))
  (Variables|Default|SetisScared true)
  (bind _outactors (Actor|GetAllActorsOfClass "/Game/MovementTestBP.MovementTestBP_C"))
  (bind _array_element (Utilities|Array|ForEachLoopwithBreak _outactors :!label _label)
    (:LoopBody
      (if (|((vectorLength((otherpos-pos)))<=radius)&&otherPos!=pos (Transformation|GetActorLocation) (Transformation|GetActorLocation _array_element) (Variables|Darkness|GetscaredRadius))
        (Variables|Default|SetisScared false)
        (goto _label Break)))))

(fn ConstructionScript
  (|CallParentFunction))